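; BP_Fireball is a fireball projectile from the Ivral boss's attack tasks, fired once at the player.
; On BeginPlay it gives its Sphere a velocity-change impulse along the look-at direction toward the player character, with no later homing.
; On hit it destroys itself, only printing debug text for the samurai or decoy.
; Any other hit counts as floor and first spawns an actor at the impact XY with a hardcoded height.
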(event EventBeginPlay
  ;[1 1 1] Gimme a title and color
  (Physics|AddImpulse (Variables|Default|GetSphere) (* (Math|Rotator|GetRotationXVector (Math|Rotator|FindLookatRotation (|GetWorldLocation>Sphere) (|GetWorldLocation>Character(Variablewhereplayer'sfeetare)))) 6e+03) "None" true))

(event Collision|EventHit
  (params (MyComp :type Primitive%20Component%20Object%20Reference) (Other :type Actor%20Object%20Reference) (OtherComp :type Primitive%20Component%20Object%20Reference) (bSelfMoved :type Boolean) (HitLocation :type Vector :default "0, 0, 0") (HitNormal :type Vector :default "0, 0, 0") (NormalImpulse :type Vector :default "0, 0, 0") (Hit :type Hit%20Result%20Structure%20%28by%20ref%29))
  (bind (_x _y) (Math|Vector|BreakVector HitLocation))
  ;[1 1 1] Gimme a title a color
  (Utilities|Casting|CastToBP_Samurai Other
    (:then
      (Development|PrintString "Hit Player")
      (Actor|DestroyActor))
    (:CastFailed
      (Utilities|Casting|CastToBP_Decoy Other
        (:then
          (Development|PrintString "(FireBall_BP) Hit Decoy")
          (Actor|DestroyActor))
        (:CastFailed
          (Development|PrintString "Hit Floor")
          (Game|SpawnActorfromClass "/Game/Bosses/Ivral/BP/AttackTasks/FireBall/AoEFireBall.AoEFireBall_C" (Math|Conversions|ToTransform(Vector) (Math|Vector|MakeVector _x _y 316.0)) "AlwaysSpawn" 0 0)
          (Actor|DestroyActor))))))

(fn ConstructionScript)