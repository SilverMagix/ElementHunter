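; Ice floor hazard actor for Ivral's boss ice attack that affects the player samurai standing on it.
; Begin and end overlap events toggle the samurai's slippery state.
; Tick calls TickDamage with a zero argument while the cached player overlaps the IceFloor component.
; Tick also destroys the actor if Timer minus delta time reaches zero, but never writes the decremented value back to Timer.
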(event EventBeginPlay
  (bind _asbp_samurai (Utilities|Casting|CastToBP_Samurai (Game|GetPlayerCharacter 0)))
  (Variables|Default|SetSamurai _asbp_samurai))

(event Collision|EventActorBeginOverlap
  (params (OtherActor :type Actor%20Object%20Reference))
  (bind _asbp_samurai (Utilities|Casting|CastToBP_Samurai OtherActor))
  (Default|SetSlippery _asbp_samurai true))

(event EventTick
  (params (DeltaSeconds :type Float%20%28single-precision%29))
  (if (Collision|IsOverlappingActor (Variables|Default|GetIceFloor) (Variables|Default|GetSamurai) :!class /Script/Engine.PrimitiveComponent)
    (Default|TickDamage (Variables|Default|GetSamurai) 0.0))
  (if (<= (- (Variables|Default|GetTimer) DeltaSeconds) 0.0)
    (Actor|DestroyActor)))

(event Collision|EventActorEndOverlap
  (params (OtherActor :type Actor%20Object%20Reference))
  (bind _asbp_samurai (Utilities|Casting|CastToBP_Samurai OtherActor))
  (Default|SetSlippery _asbp_samurai false))

(fn ConstructionScript)