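; BP_Slash is a sword slash actor that damages Irval on overlap.
; When it overlaps an IrvalPawnC, it calls HitIrval with the slash damage, spawns a hit particle effect at its Box component and destroys itself.
; Tick accumulates the slash's lifetime and destroys the actor once MaxTimer is reached, so missed slashes expire.
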(event EventBeginPlay)

(event Collision|EventActorBeginOverlap
  (params (OtherActor :type Actor%20Object%20Reference))
  ;[1 1 1] When Slash hits Irval
  (bind _asirval_pawn_c (Utilities|Casting|CastToIrvalPawnC OtherActor))
  (Class|IrvalPawnC|HitIrval _asirval_pawn_c (Variables|Default|GetSwordSlash%20Damage))
  (Effects|SpawnEmitteratLocation (Variables|Default|GetHitFix) (Transformation|GetWorldLocation (Variables|Default|GetBox)))
  (Actor|DestroyActor))

(event EventTick
  (params (DeltaSeconds :type Float%20%28single-precision%29))
  ;[1 1 1] Decay over time
  (bind _output_get (Variables|Default|SetLife (+ DeltaSeconds (Variables|Default|GetLife))))
  (if (>= _output_get (Variables|Default|GetMaxTimer))
    (Actor|DestroyActor)))

(fn ConstructionScript)