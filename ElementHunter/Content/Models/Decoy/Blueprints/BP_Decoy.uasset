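; BP_Decoy is a decoy actor that is destroyed when an IrvalPawnC touches it and notifies the player of the hit.
; It caches all IrvalPawnC actors on BeginPlay, then checks each for overlap every Tick instead of using overlap events.
; On a hit it prints a debug message, sets DecoyHasBeenHit on the player's BP_Samurai, breaks the loop and destroys itself.
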(event Custom|Break
  (Utilities|Array|ForEachLoopwithBreak (Variables|Default|GetIrval)) ; enters at Break
)

(event EventBeginPlay
  (bind _outactors (Actor|GetAllActorsOfClass "/Script/ElementHunter.IrvalPawnC"))
  (Variables|Default|SetIrval _outactors))

(event Collision|EventActorBeginOverlap
  (params (OtherActor :type Actor%20Object%20Reference)))

(event EventTick
  (params (DeltaSeconds :type Float%20%28single-precision%29))
  (bind _array_element (Utilities|Array|ForEachLoopwithBreak (Variables|Default|GetIrval))
    (:LoopBody
      (if (Collision|IsOverlappingActor _array_element :!class /Script/Engine.Actor)
        (Development|PrintString "(BP_Decoy) Decoy has been hit")
        (CallFunction|IsHit)
        (CallFunction|Break)
        (Actor|DestroyActor)))))

(fn ConstructionScript)

(fn IsHit
  (bind _asbp_samurai (Utilities|Casting|CastToBP_Samurai (Game|GetPlayerCharacter 0)))
  (Variables|/Game/Models/MainCharacter/Blueprints/BP_Samurai.BP_Samurai_C|SetDecoyHasBeenHit _asbp_samurai true))